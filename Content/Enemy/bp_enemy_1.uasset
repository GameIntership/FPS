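; Enemy character Blueprint that carries a weapon, plays a montage attack and dies when its health runs out.
; On BeginPlay it spawns Wepon_1 and snaps it to the hand_rSocket on its mesh.
; The attack event plays the attack montage and fires Onattackfinished whether it completes or is interrupted.
; Tick polls Health every frame and destroys the actor at zero or below.
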(event Custom|attack
  (Animation|Montage|PlayMontage (Variables|Character|GetMesh) "/Game/Enemy/Attack/attack_anim_montage.attack_anim_montage"
    (:OnCompleted
      _)
    (:OnInterrupted
      _))
  (Default|CallOnattackfinished))

(event Custom|wepon
  (bind _returnvalue (Game|SpawnActorfromClass "/Game/Enemy/Weapon/wepon_1.wepon_1_C" (Transformation|GetActorTransform) "Undefined" "MultiplyWithRoot" 0 0))
  (Transformation|AttachComponentToComponent _returnvalue (Variables|Character|GetMesh) "hand_rSocket" "SnapToTarget" "SnapToTarget" "SnapToTarget" true))

(event EventBeginPlay
  (CallFunction|Wepon))

(event EventTick
  (params (DeltaSeconds :type Float%20%28single-precision%29))
  (if (>= 0 (Variables|Default|Gethealth))
    (Actor|DestroyActor)))

(fn ConstructionScript)