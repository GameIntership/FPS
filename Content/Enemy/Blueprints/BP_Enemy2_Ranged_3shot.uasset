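; Ranged enemy that turns toward the player and fires BP_EnemyBullet from an arrow component.
; AI Perception sets FoundPlayer, which allows firing; losing sight, or a BP_Bullet hit while unaware, triggers an AI move toward the player.
; Tick makes staggered Shoot calls, each re-aiming at the player even when unseen, while a shared CanAttack cooldown gates the actual shots.
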(event OnSeePawn(PawnSensing)
  (params (Pawn :type Pawn%20Object%20Reference))
  ;[0.8426 0.9821 1] see
  (Utilities|Casting|CastToBP_FirstPersonCharacter Pawn))

(event OnTargetPerceptionUpdated(AIPerception)
  (params (Actor :type Actor%20Object%20Reference) (Stimulus :type AI%20Stimulus%20Structure))
  ;[0.8426 0.9821 1] see
  (bind _asbp_first_person_character (Utilities|Casting|CastToBP_FirstPersonCharacter Actor))
  (if (.bsuccessfullysensed Stimulus)
    (Transformation|SetActorRotation (Math|Rotator|FindRelativeLookatRotation (Math|Conversions|ToTransform(Vector) (Transformation|GetActorLocation)) (Transformation|GetActorLocation _asbp_first_person_character)))
    (Variables|Default|Setfound%20player true)
    (else
      (Variables|Default|Setfound%20player false)
      (Variables|Default|SetlookingForPlayer true))))

(event Custom|attack
  ;[1 1 1] shoot logic
  (Game|SpawnActorfromClass "/Game/Enemy/Blueprints/BP_EnemyBullet.BP_EnemyBullet_C" (Transformation|GetWorldTransform (Variables|Default|GetArrow1)) "Undefined" "MultiplyWithRoot" 0 0))

(event Custom|shoot
  ;[1 1 1] shoot logic
  (Transformation|SetActorRotation (Math|Rotator|FindRelativeLookatRotation (Math|Conversions|ToTransform(Vector) (Transformation|GetActorLocation)) (Transformation|GetActorLocation (Game|GetPlayerCharacter 0))))
  (if (Variables|Default|Getfound%20player)
    (if (Variables|Default|GetCanAttack)
      (Variables|Default|SetCanAttack false)
      (CallFunction|Attack)
      (Utilities|FlowControl|Delay 1.0)
      (Variables|Default|SetCanAttack true))))

(event Custom|look%20for%20player
  ;[1 1 1] move to player when lost
  (if (Variables|Default|GetlookingForPlayer)
    (Variables|Default|SetlookingForPlayer false)
    (AI|AIMoveTo self "0, 0, 0" (Game|GetPlayerCharacter 0) 4e+02 false)))

(event Collision|EventHit
  (params (MyComp :type Primitive%20Component%20Object%20Reference) (Other :type Actor%20Object%20Reference) (OtherComp :type Primitive%20Component%20Object%20Reference) (bSelfMoved :type Boolean) (HitLocation :type Vector :default "0, 0, 0") (HitNormal :type Vector :default "0, 0, 0") (NormalImpulse :type Vector :default "0, 0, 0") (Hit :type Hit%20Result%20Structure%20%28by%20ref%29))
  ;[1 1 1] to found player by bing hited
  (Utilities|Casting|CastToBP_Bullet Other)
  (if (not (Variables|Default|Getfound%20player))
    (Variables|Default|SetlookingForPlayer true)))

(event EventDestroyed
  (Utilities|FlowControl|Delay 1.0)
  (CallFunction|Shoot))

(event EventTick
  (params (DeltaSeconds :type Float%20%28single-precision%29))
  (Utilities|FlowControl|Sequence
    (:then_0
      (CallFunction|Shoot)
      (Utilities|FlowControl|Delay 0.2)
      (CallFunction|Shoot)
      (Utilities|FlowControl|Delay 0.2)
      (CallFunction|Shoot))
    (:then_1
      (CallFunction|LookforPlayer))))

(fn ConstructionScript)