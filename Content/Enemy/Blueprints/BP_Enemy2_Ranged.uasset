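; BP_Enemy2_Ranged is a ranged enemy that turns toward the player and shoots when it sees them.
; Its PawnSensing sight event filters for BP_FirstPersonCharacter and snaps the actor's rotation to look at that character's location.
; If CanAttack is true, it then spawns a BP_EnemyBullet at the Arrow1 component's world transform; this graph never changes that flag.
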(event OnSeePawn(PawnSensing)
  (params (Pawn :type Pawn%20Object%20Reference))
  (bind _asbp_first_person_character (Utilities|Casting|CastToBP_FirstPersonCharacter Pawn))
  (Transformation|SetActorRotation (Math|Rotator|FindRelativeLookatRotation (Math|Conversions|ToTransform(Vector) (Transformation|GetActorLocation)) (Transformation|GetActorLocation _asbp_first_person_character)))
  (if (Variables|Default|GetCanAttack)
    (Game|SpawnActorfromClass "/Game/Enemy/Blueprints/BP_EnemyBullet.BP_EnemyBullet_C" (Transformation|GetWorldTransform (Variables|Default|GetArrow1)) "Undefined" "MultiplyWithRoot" 0 0)))

(fn ConstructionScript)