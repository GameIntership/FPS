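; Level exit portal that loads the NextLevel map when the player presses Interact while standing inside its Box trigger.
; Box overlaps with BP_FirstPersonCharacter enable or disable the portal's input and open or close a Gate guarding the Interact action.
; After requesting the level load, it hides the mouse cursor and switches to game-only input.
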(event OnComponentEndOverlap(Box)
  (params (OverlappedComponent :type Primitive%20Component%20Object%20Reference) (OtherActor :type Actor%20Object%20Reference) (OtherComp :type Primitive%20Component%20Object%20Reference) (OtherBodyIndex :type Integer))
  (bind _returnvalue (Game|GetPlayerController 0))
  ;[0.2052 0.2052 0.2052] Active Interact Input when ever the character is close to the Portal
  (Utilities|Casting|CastToBP_FirstPersonCharacter OtherActor)
  (Input|DisableInput (Game|GetPlayerController 0))
  (Utilities|FlowControl|Gate true) ; enters at Close
)

(event OnComponentBeginOverlap(Box)
  (params (OverlappedComponent :type Primitive%20Component%20Object%20Reference) (OtherActor :type Actor%20Object%20Reference) (OtherComp :type Primitive%20Component%20Object%20Reference) (OtherBodyIndex :type Integer) (bFromSweep :type Boolean) (SweepResult :type Hit%20Result%20Structure%20%28by%20ref%29))
  (bind _returnvalue (Game|GetPlayerController 0))
  ;[0.2052 0.2052 0.2052] Active Interact Input when ever the character is close to the Portal
  (Utilities|Casting|CastToBP_FirstPersonCharacter OtherActor)
  (Input|EnableInput (Game|GetPlayerController 0))
  (Utilities|FlowControl|Gate true) ; enters at Open
)

(event Input|ActionEvents|InputActionInteract
  (params (Key :type Key%20Structure :default "None"))
  (bind _returnvalue (Game|GetPlayerController 0))
  ;[0.2052 0.2052 0.2052] Active Interact Input when ever the character is close to the Portal
  (:Pressed
    (Utilities|FlowControl|Gate true
      (:Exit
        ;[0.2052 0.2052 0.2052] Open Next Level
        (Game|OpenLevel(byObjectReference) (Variables|Default|GetNextLevel))
        (Variables|/Script/Engine.PlayerController|SetbShowMouseCursor _returnvalue false)
        (Input|SetInputModeGameOnly _returnvalue false)))))

(fn ConstructionScript)