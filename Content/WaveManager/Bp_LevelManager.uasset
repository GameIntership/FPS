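; Level manager actor that tracks wave progression and decides what happens when a level's waves run out.
; On BeginPlay it binds its Spawn event to the first-person game mode's new-wave notification.
; Each Spawn advances the wave counter and shows a wave popup while waves remain.
; Otherwise it shows the win screen on the last level, or spawns a next-level portal at its own transform.
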(event Custom|Spawn
  ;[0.2052 0.2052 0.2052] Check we have remaning wave
  (if (< (Variables|Default|GetCurrentWave) (Variables|Default|GetWaveCount))
    ;[0.2052 0.2052 0.2052] Display the Next Wave wedget
    (Math|Integer|IncrementInt (Variables|Default|GetCurrentWave)
      (:%20%20
        (bind _returnvalue (UserInterface|CreateWidget "/Game/WaveManager/Wb_WavePopUp.Wb_WavePopUp_C"))
        (Default|SetText _returnvalue (Variables|Default|GetWaveCount) (Variables|Default|GetCurrentWave))
        (UserInterface|Viewport|AddtoViewport _returnvalue 0)))
    (elif (Variables|Default|GetIsLastLevel)
      ;[0.2052 0.2052 0.2052] Display the winning widget
      (bind _returnvalue_2 (UserInterface|CreateWidget "/Game/WaveManager/Wb_FinishGame.Wb_FinishGame_C"))
      (Default|Win _returnvalue_2)
      (UserInterface|Viewport|AddtoViewport _returnvalue_2 0)
      (else
        ;[0.2052 0.2052 0.2052] Spawn Next Level Portal
        (bind _returnvalue_3 (Game|SpawnActorfromClass "/Game/WaveManager/Bp_NextLevelPortal.Bp_NextLevelPortal_C" (Transformation|GetActorTransform) "AlwaysSpawn" "MultiplyWithRoot" 0 0))
        (Variables|/Game/WaveManager/Bp_NextLevelPortal.Bp_NextLevelPortal_C|SetNextLevel _returnvalue_3 (Variables|Default|GetNext%20Level))))))

(event EventBeginPlay
  ;[0.2052 0.2052 0.2052] Bind spawn Event
  (bind _asbp_first_person_game_mode (Utilities|Casting|CastToBP_FirstPersonGameMode (Game|GetGameMode)))
  (EventDispatchers|BindEventtoSpawnNewWave _asbp_first_person_game_mode (delegate Custom|Spawn)))

(fn ConstructionScript)